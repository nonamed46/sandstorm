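; StarConstellation_BP is a star constellation decal that can be lit up when a message reaches it.
; BeginPlay creates a dynamic material instance on the decal, and MSGShowStars raises its EmissiveStrength to make the stars glow.
; A box overlap passes this actor to any Interaction_BPI implementer through MSGSetStarDecalMessage, and clears that reference when the overlap ends.
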(event OnComponentBeginOverlap(Box)
  (params (OverlappedComponent :type Primitive%20Component%20Object%20Reference) (OtherActor :type Actor%20Object%20Reference) (OtherComp :type Primitive%20Component%20Object%20Reference) (OtherBodyIndex :type Integer) (bFromSweep :type Boolean) (SweepResult :type Hit%20Result%20Structure%20%28by%20ref%29))
  (if (Utilities|DoesObjectImplementInterface OtherActor "/Game/Blueprints/Interaction_BPI.Interaction_BPI_C")
    (Class|InteractionBPI|MSGSetStarDecal(Message) OtherActor self)
    (Development|PrintString "Adding Decal to Player")))

(event OnComponentEndOverlap(Box)
  (params (OverlappedComponent :type Primitive%20Component%20Object%20Reference) (OtherActor :type Actor%20Object%20Reference) (OtherComp :type Primitive%20Component%20Object%20Reference) (OtherBodyIndex :type Integer))
  (if (Utilities|DoesObjectImplementInterface OtherActor "/Game/Blueprints/Interaction_BPI.Interaction_BPI_C")
    (Class|InteractionBPI|MSGSetStarDecal(Message) OtherActor)))

(event EventBeginPlay
  (bind _returnvalue (Rendering|Material|CreateDynamicMaterialInstance (Variables|Default|GetDecal) :!class /Script/Engine.DecalComponent)))

(event EventMSGShowStars
  (Rendering|Material|SetScalarParameterValue (stale EventBeginPlay _returnvalue) "EmissiveStrength" 2e+01 :!class /Script/Engine.MaterialInstanceDynamic)
  (Development|PrintString "Showing Stars"))

(fn ConstructionScript)