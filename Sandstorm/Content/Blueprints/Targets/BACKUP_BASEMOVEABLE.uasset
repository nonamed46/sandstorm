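; Base moveable target actor that slides between its placed position and a configurable XYZ offset when it receives begin-task and end-task messages.
; Looping timers tick the ascend or descend movement, with gates and timer resets stopping the opposing direction.
; Each tick steps along the normalized direction by Speed, clamped per axis between start and end.
; A sound plays during movement and stops on arrival at either end.
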(event Custom|Ascend
  (bind _self self)
  (bind _endpos (Variables|Default|GetEndPos))
  (bind _speed (Variables|Default|GetSpeed))
  (bind _direction (Variables|Default|GetDirection))
  (bind _startpos (Variables|Default|GetStartPos))
  (bind _returnvalue (Transformation|GetActorLocation _self))
  (bind _returnvalue_2 (* _direction _speed))
  ;[0.1729 1 0.3234] Begin Task /Ascend. Start Sound, Looping Timer, Stop opposing Movement, Close Opposing Gate
  ;[1 0.7769 0] Move Actor in Direction by Speed, Clamped by Max Position(set in E. Begin Play)
  (Utilities|FlowControl|Gate true
    (:Exit
      (Transformation|SetActorLocation _self (Math|Vector|MakeVector (Math|Float|Clamp(Float) (+ (.x _returnvalue) (.x _returnvalue_2)) (.x _startpos) (.x _endpos)) (Math|Float|Clamp(Float) (+ (.y _returnvalue) (.y _returnvalue_2)) (.y _startpos) (.y _endpos)) (Math|Float|Clamp(Float) (+ (.z _returnvalue) (.z _returnvalue_2)) (.z _startpos) (.z _endpos))) false false)
      ;[0.1362 0.1893 1] If Target/Start is reached Stop ticking
      (if (Math|Vector|Equal(Vector) (Transformation|GetActorLocation self) (Variables|Default|GetEndPos) 0.002)
        (Utilities|Time|SetTimerbyEvent (EventDispatchers|CreateEvent :!event Custom|Ascend) 0.0)
        ;[1 0.2247 0.991] Stop Sound
        (Audio|Components|Audio|Stop (Variables|Default|GetAudio))))))

(event Custom|Descend
  (bind _self self)
  (bind _direction (Variables|Default|GetDirection))
  (bind _startpos (Variables|Default|GetStartPos))
  (bind _endpos (Variables|Default|GetEndPos))
  (bind _speed (Variables|Default|GetSpeed))
  (bind _returnvalue (Transformation|GetActorLocation _self))
  (bind _returnvalue_2 (* _direction _speed))
  ;[1 0.103 0.0831] End Task / Descend (see above similar to ascend)
  ;[1 0.7769 0] Move Actor in Direction by Speed, Clamped by Max Position(set in E. Begin Play)
  (Utilities|FlowControl|Gate true
    (:Exit
      (Transformation|SetActorLocation _self (Math|Vector|MakeVector (Math|Float|Clamp(Float) (- (.x _returnvalue) (.x _returnvalue_2)) (.x _startpos) (.x _endpos)) (Math|Float|Clamp(Float) (- (.y _returnvalue) (.y _returnvalue_2)) (.y _startpos) (.y _endpos)) (Math|Float|Clamp(Float) (- (.z _returnvalue) (.z _returnvalue_2)) (.z _startpos) (.z _endpos))) false false)
      ;[0.1362 0.1893 1] If Target/Start is reached Stop ticking
      (if (Math|Vector|Equal(Vector) (Transformation|GetActorLocation self) (Variables|Default|GetStartPos) 0.002)
        (Utilities|Time|SetTimerbyEvent (EventDispatchers|CreateEvent :!event Custom|Descend) 0.0)
        ;[1 0.2247 0.991] Stop Sound
        (Audio|Components|Audio|Stop (Variables|Default|GetAudio))))))

(event EventMSGBeginTask
  (params (time :type Float%20%28single-precision%29))
  (bind _self self)
  (bind _self_2 self)
  (bind _endpos (Variables|Default|GetEndPos))
  (bind _direction (Variables|Default|GetDirection))
  (bind _speed (Variables|Default|GetSpeed))
  (bind _direction_2 (Variables|Default|GetDirection))
  (bind _audio (Variables|Default|GetAudio))
  (bind _startpos (Variables|Default|GetStartPos))
  (bind _endpos_2 (Variables|Default|GetEndPos))
  (bind _speed_2 (Variables|Default|GetSpeed))
  (bind _startpos_2 (Variables|Default|GetStartPos))
  (bind _returnvalue (Transformation|GetActorLocation _self))
  (bind _returnvalue_2 (Transformation|GetActorLocation _self_2))
  (bind _returnvalue_3 (* _direction _speed_2))
  (bind _returnvalue_4 (* _direction_2 _speed))
  ;[0.1729 1 0.3234] Begin Task /Ascend. Start Sound, Looping Timer, Stop opposing Movement, Close Opposing Gate
  (Utilities|Time|SetTimerbyEvent (delegate Custom|Ascend) 0.02 true)
  (Utilities|FlowControl|Sequence
    (:then_0
      ;[1 1 1] Stop Opposing Movement
      (Utilities|Time|SetTimerbyEvent (EventDispatchers|CreateEvent :!event Custom|Descend) 0.0))
    (:then_1
      ;[1 0.7769 0] Move Actor in Direction by Speed, Clamped by Max Position(set in E. Begin Play)
      (Utilities|FlowControl|Gate true) ; enters at Open
    )
    (:then_2
      (Utilities|FlowControl|Gate true) ; enters at Close
    )
    (:then_3
      ;[1 0.2247 0.991] BeginSound or continue playing
      (if (not (Audio|Components|Audio|IsPlaying _audio))
        (Audio|Components|Audio|Play _audio 0.0)))))

(event EventBeginPlay
  (bind _self self)
  (bind _returnvalue (Transformation|GetActorLocation _self))
  ;[1 1 1] Begin Play: Set Start and End Position based on Max Offset in X,Y and Z Direction
  (bind _output_get (Variables|Default|SetStartPos (Math|Vector|MakeVector (.x _returnvalue) (.y _returnvalue) (.z _returnvalue))))
  (bind _output_get_2 (Variables|Default|SetEndPos (Math|Vector|MakeVector (+ (.x _returnvalue) (Variables|Default|GetMax_X-Offset)) (+ (.y _returnvalue) (Variables|Default|GetMax_Y-Offset)) (+ (.z _returnvalue) (Variables|Default|GetMax_Z-Offset)))))
  (Variables|Default|SetDirection (Math|Vector|Normalize (- _output_get_2 _output_get))))

(event EventMSGEndTask
  (bind _self self)
  (bind _self_2 self)
  (bind _endpos (Variables|Default|GetEndPos))
  (bind _direction (Variables|Default|GetDirection))
  (bind _speed (Variables|Default|GetSpeed))
  (bind _direction_2 (Variables|Default|GetDirection))
  (bind _audio (Variables|Default|GetAudio))
  (bind _startpos (Variables|Default|GetStartPos))
  (bind _endpos_2 (Variables|Default|GetEndPos))
  (bind _speed_2 (Variables|Default|GetSpeed))
  (bind _startpos_2 (Variables|Default|GetStartPos))
  (bind _returnvalue (Transformation|GetActorLocation _self))
  (bind _returnvalue_2 (Transformation|GetActorLocation _self_2))
  (bind _returnvalue_3 (* _direction _speed_2))
  (bind _returnvalue_4 (* _direction_2 _speed))
  ;[1 0.103 0.0831] End Task / Descend (see above similar to ascend)
  (Utilities|Time|SetTimerbyEvent (delegate Custom|Descend) 0.02 true)
  (Utilities|FlowControl|Sequence
    (:then_0
      ;[1 0.2247 0.991] BeginSound or continue playing
      (if (not (Audio|Components|Audio|IsPlaying _audio))
        (Audio|Components|Audio|Play _audio 0.0)))
    (:then_1
      ;[1 0.7769 0] Move Actor in Direction by Speed, Clamped by Max Position(set in E. Begin Play)
      (Utilities|FlowControl|Gate true) ; enters at Close
    )
    (:then_2
      (Utilities|FlowControl|Gate true) ; enters at Open
    )
    (:then_3
      ;[1 1 1] Stop Opposing Movement
      (Utilities|Time|SetTimerbyEvent (EventDispatchers|CreateEvent :!event Custom|Ascend) 0.0))))

(fn ConstructionScript
  (|CallParentFunction))