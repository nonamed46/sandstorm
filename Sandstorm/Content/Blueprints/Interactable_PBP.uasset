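; Base interactable Blueprint that lets overlapping actors interact with it and can start or stop a task on a Target.
; Its Trigger sets or clears it as the overlapping actor's interactable through Interaction_BPI.
; MSGInteract calls an empty Interaction event, which serves as a hook for specific behavior.
; StartTargetTask and StopTargetTask message the Target through Target_BPI, printing debug errors if it is invalid or lacks the interface.
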(event OnComponentBeginOverlap(Trigger)
  (params (OverlappedComponent :type Primitive%20Component%20Object%20Reference) (OtherActor :type Actor%20Object%20Reference) (OtherComp :type Primitive%20Component%20Object%20Reference) (OtherBodyIndex :type Integer) (bFromSweep :type Boolean) (SweepResult :type Hit%20Result%20Structure%20%28by%20ref%29))
  ;[0 1 0.1527] When Player starts/stops Overlapping set/reset self as Target
  (if (Utilities|DoesObjectImplementInterface OtherActor "/Game/Blueprints/Interaction_BPI.Interaction_BPI_C")
    (Class|InteractionBPI|MSGSetInteractable(Message) OtherActor self)))

(event OnComponentEndOverlap(Trigger)
  (params (OverlappedComponent :type Primitive%20Component%20Object%20Reference) (OtherActor :type Actor%20Object%20Reference) (OtherComp :type Primitive%20Component%20Object%20Reference) (OtherBodyIndex :type Integer))
  ;[0 1 0.1527] When Player starts/stops Overlapping set/reset self as Target
  (if (Utilities|DoesObjectImplementInterface OtherActor "/Game/Blueprints/Interaction_BPI.Interaction_BPI_C")
    (Class|InteractionBPI|MSGSetInteractable(Message) OtherActor)))

(event Custom|Interaction)

(event Custom|StopTargetTask
  (bind _target (Variables|Default|GetTarget))
  (bind _returnvalue (Utilities|IsValid _target))
  (bind _returnvalue_2 (Utilities|DoesObjectImplementInterface _target "/Game/Blueprints/Target_BPI.Target_BPI_C"))
  ;[1 1 1] Start Targets Task
  (if (and _returnvalue _returnvalue_2)
    (Class|TargetBPI|MSGEndTask(Message) _target)
    (else
      ;;[1 0.5 0] Debug, Throw Error
      (Development|PrintString (Utilities|String|Append "Error Stopping Task" "target is valid?" (Utilities|String|ToString(Boolean) _returnvalue)) true true "(R=1.000000,G=0.009271,B=0.000000,A=1.000000)" 2e+01)
      (Development|PrintString (Utilities|String|Append "Target Implements Interface?" (Utilities|String|ToString(Boolean) _returnvalue_2)) true true "(R=1.000000,G=0.010417,B=0.010417,A=1.000000)" 2e+01))))

(event Custom|StartTargetTask
  (bind _target (Variables|Default|GetTarget))
  (bind _returnvalue (Utilities|IsValid _target))
  (bind _returnvalue_2 (Utilities|DoesObjectImplementInterface _target "/Game/Blueprints/Target_BPI.Target_BPI_C"))
  ;[1 1 1] Start Targets Task
  (if (and _returnvalue _returnvalue_2)
    (Development|PrintString "Successful Cast")
    (Class|TargetBPI|MSGBeginTask(Message) _target 0.0)
    (else
      ;;[1 0.5 0] Debug, Throw Error
      (Development|PrintString (Utilities|String|Append "Error Starting Task:" "target is valid?" (Utilities|String|ToString(Boolean) _returnvalue)) true true "(R=1.000000,G=0.048679,B=0.000000,A=1.000000)" 2e+01)
      (Development|PrintString (Utilities|String|Append "Implements Interface?" (Utilities|String|ToString(Boolean) _returnvalue_2)) true true "(R=1.000000,G=0.086574,B=0.000000,A=1.000000)" 2e+01))))

(event EventMSGInteract
  (CallFunction|Interaction))

(fn ConstructionScript)