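; Interactable lever Blueprint that signals a target when used, then resets itself automatically.
; Interaction passes a DoOnce gate, sends a begin-task message to Target, rotates the Switch pitch with the RotUp timeline and starts a timer.
; When the timer fires, ResetLever sends the end-task message and plays RotDown, reopening the gate shortly after the rotation finishes.
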(event Custom|ResetLever
  (Class|TargetBPI|MSGEndTask(Message) (Variables|Default|GetTarget))
  (bind _yrot (Timeline|RotDown PlayFromStart)
    (:Update
      (Transformation|SetRelativeRotation (Variables|Default|GetSwitch) (Math|Rotator|MakeRotator 0.0 _yrot 0.0) false false))
    (:Finished
      (Utilities|FlowControl|Delay 0.5)
      (Utilities|FlowControl|DoOnce false) ; enters at Reset
    )))

(event EventInteraction
  (Utilities|FlowControl|DoOnce false
    (:Completed
      (Class|TargetBPI|MSGBeginTask(Message) (Variables|Default|GetTarget) 0.0)
      (Utilities|Time|SetTimerbyEvent (delegate Custom|ResetLever) 1.5)
      (bind _yrot (Timeline|RotUp PlayFromStart)
        (:Update
          (Transformation|SetRelativeRotation (Variables|Default|GetSwitch) (Math|Rotator|MakeRotator 0.0 _yrot 0.0) false false))))))

(fn ConstructionScript
  (|CallParentFunction))