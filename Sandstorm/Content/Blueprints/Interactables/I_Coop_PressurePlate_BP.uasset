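; Co-op pressure plate interactable that starts its target task while at least two fox characters stand on it.
; Overlaps on PressureCheck count actors that implement Interaction_BPI and are of class Big or Small.
; Reaching a count of two calls StartTargetTask, while any counted fox leaving decrements the count and calls StopTargetTask without checking the remainder.
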(event OnComponentBeginOverlap(PressureCheck)
  (params (OverlappedComponent :type Primitive%20Component%20Object%20Reference) (OtherActor :type Actor%20Object%20Reference) (OtherComp :type Primitive%20Component%20Object%20Reference) (OtherBodyIndex :type Integer) (bFromSweep :type Boolean) (SweepResult :type Hit%20Result%20Structure%20%28by%20ref%29))
  (bind _foxcount (Variables|Default|GetfoxCount))
  (if (Utilities|DoesObjectImplementInterface OtherActor "/Game/Blueprints/Interaction_BPI.Interaction_BPI_C")
    (Utilities|Casting|CastToBig OtherActor
      (:then
        _)
      (:CastFailed
        (Utilities|Casting|CastToSmall OtherActor)))
    (Math|Integer|IncrementInt _foxcount
      (:%20%20
        (if (>= _foxcount 2)
          (CallFunction|StartTargetTask))))))

(event OnComponentEndOverlap(PressureCheck)
  (params (OverlappedComponent :type Primitive%20Component%20Object%20Reference) (OtherActor :type Actor%20Object%20Reference) (OtherComp :type Primitive%20Component%20Object%20Reference) (OtherBodyIndex :type Integer))
  (if (Utilities|DoesObjectImplementInterface OtherActor "/Game/Blueprints/Interaction_BPI.Interaction_BPI_C")
    (Utilities|Casting|CastToBig OtherActor
      (:then
        _)
      (:CastFailed
        (Utilities|Casting|CastToSmall (stale OnComponentBeginOverlap(PressureCheck) OtherActor))))
    (Math|Integer|DecrementInt (Variables|Default|GetfoxCount)
      (:%20%20
        (CallFunction|StopTargetTask)))))

(fn ConstructionScript
  (|CallParentFunction))