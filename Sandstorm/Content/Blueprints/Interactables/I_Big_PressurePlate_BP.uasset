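; A pressure plate interactable that responds only to actors of the Big class.
; Overlaps on the PressureCheck component are filtered by an Interaction_BPI interface check and a cast to Big.
; A valid actor entering calls StartTargetTask, and one leaving calls StopTargetTask, with no tracking of how many remain on the plate.
; The construction script only runs the parent's setup.
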(event OnComponentBeginOverlap(PressureCheck)
  (params (OverlappedComponent :type Primitive%20Component%20Object%20Reference) (OtherActor :type Actor%20Object%20Reference) (OtherComp :type Primitive%20Component%20Object%20Reference) (OtherBodyIndex :type Integer) (bFromSweep :type Boolean) (SweepResult :type Hit%20Result%20Structure%20%28by%20ref%29))
  (if (Utilities|DoesObjectImplementInterface OtherActor "/Game/Blueprints/Interaction_BPI.Interaction_BPI_C")
    (Utilities|Casting|CastToBig OtherActor)
    (CallFunction|StartTargetTask)))

(event OnComponentEndOverlap(PressureCheck)
  (params (OverlappedComponent :type Primitive%20Component%20Object%20Reference) (OtherActor :type Actor%20Object%20Reference) (OtherComp :type Primitive%20Component%20Object%20Reference) (OtherBodyIndex :type Integer))
  (if (Utilities|DoesObjectImplementInterface OtherActor "/Game/Blueprints/Interaction_BPI.Interaction_BPI_C")
    (Utilities|Casting|CastToBig OtherActor)
    (CallFunction|StopTargetTask)))

(fn ConstructionScript
  (|CallParentFunction))